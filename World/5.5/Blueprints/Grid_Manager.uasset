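; Grid manager that streams terrain chunks in a square radius around the player, with resolution based on distance.
; A looping timer runs Calc_Grid, which on chunk changes asks MyChunkGenerator for new or LOD-outdated chunks and despawns out-of-range ones.
; SpawnChunk turns mesh data into AsyncPMC components, with collision only at one vertex count, and replaces chunks queued for update.
; Parallel arrays track each chunk's coordinates, LOD and component.
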(event EventBeginPlay
  (bind _my_chunk_generator (Variables|Default|GetMy_Chunk_Generator))
  (EventDispatchers|BindEventtoOnChunkGenerated _my_chunk_generator (EventDispatchers|CreateEvent :!event SpawnChunk))
  (Utilities|Time|SetTimerbyFunctionName 0 "Calc_Grid" 0.5 true true 0.1)
  (Variables|/Script/Landscape_proj.Chunk_Generator_Component|SetChunkSize _my_chunk_generator (.x (Variables|Default|GetChunk_Size))))

(event Collision|EventActorBeginOverlap
  (params (OtherActor :type Actor%20Object%20Reference)))

(event EventTick
  (params (DeltaSeconds :type Float%20%28single-precision%29)))

(fn ConstructionScript)

(fn CalcGrid
  (bind _returnvalue (Class|KismetSystemLibrary|MakeLiteralInteger 2))
  (bind _chunk_size (Variables|Default|GetChunk_Size))
  (bind _player (Variables|Components|GetPlayer))
  (bind _chunk_radius (Variables|Default|GetChunk_Radius))
  (bind _my_chunk_generator (Variables|Default|GetMy_Chunk_Generator))
  (bind _chunk_radius_2 (Variables|Default|GetChunk_Radius))
  (bind _chunk_size_2 (Variables|Default|GetChunk_Size))
  (bind _chunk_radius_3 (Variables|Default|GetChunk_Radius))
  (bind _chunk_radius_4 (Variables|Default|GetChunk_Radius))
  (bind _chunk_radius_5 (Variables|Default|GetChunk_Radius))
  (bind _returnvalue_2 (Transformation|GetActorLocation _player))
  (bind (_x _y) (Math|Vector2D|BreakVector2D _chunk_size))
  (bind _returnvalue_3 (* _chunk_radius -1))
  (bind _returnvalue_4 (* _chunk_radius_4 -1))
  (bind _returnvalue_5 (* _chunk_radius_2 2))
  (bind _returnvalue_6 (+ _returnvalue_5 1))
  (bind _returnvalue_7 (/ (.x _returnvalue_2) _x))
  (bind _returnvalue_8 (/ (.y _returnvalue_2) _y))
  (bind _returnvalue_9 (Math|Float|Floor _returnvalue_7))
  (bind _returnvalue_10 (Math|Float|Floor _returnvalue_8))
  (bind _returnvalue_11 (Math|Conversions|ToFloat(Integer) _returnvalue_10))
  (bind _returnvalue_12 (Math|Conversions|ToFloat(Integer) _returnvalue_9))
  (bind _returnvalue_13 (Math|Vector2D|MakeVector2D _returnvalue_12 _returnvalue_11))
  (bind (_x_2 _y_2) (Math|Vector2D|BreakVector2D _returnvalue_13))
  (bind (_x_3 _y_3) (Math|Vector2D|BreakVector2D _returnvalue_13))
  (bind (_x_4 _y_4) (Math|Vector2D|BreakVector2D _returnvalue_13))
  (bind _returnvalue_14 (Math|Float|Floor _x_4))
  (bind _returnvalue_15 (Math|Float|Floor _y_4))
  (bind _returnvalue_16 (- _returnvalue_14 _chunk_radius_5))
  (bind _returnvalue_17 (- _returnvalue_15 _chunk_radius_5))
  (bind _returnvalue_18 (+ _chunk_radius_5 _returnvalue_14))
  (bind _returnvalue_19 (+ _chunk_radius_5 _returnvalue_15))
  (Utilities|FlowControl|Sequence
    (:then_0
      (if (not (Utilities|Operators|EqualEqual (Variables|Default|GetCurrent_Chunk) _returnvalue_13 0.0))
        (if (Utilities|Operators|EqualEqual (Variables|Default|GetCurrent_Chunk) "(X=0.500000,Y=0.500000)" 0.0)
          ;[1 0.5833 0.5833] Default Chunk Spawns aka Init
          (for _index (range _returnvalue_4 _chunk_radius_4) :!label _label
            (for _index_2 (range _returnvalue_4 _chunk_radius_4)
              (Class|ChunkGeneratorComponent|GenerateChunk _my_chunk_generator (+ (Math|Float|Floor _x_3) _index) (+ (Math|Float|Floor _y_3) _index_2) (Math|Integer|SelectInt (Math|Integer|SelectInt (Math|Integer|Absolute(Integer) (Math|Float|Floor (- _x_3 (Math|Conversions|ToFloat(Integer) _index)))) (Math|Integer|Absolute(Integer) (Math|Float|Floor (- _y_3 (Math|Conversions|ToFloat(Integer) _index_2)))) (> (Math|Integer|Absolute(Integer) (Math|Float|Floor (- _x_3 (Math|Conversions|ToFloat(Integer) _index)))) (Math|Integer|Absolute(Integer) (Math|Float|Floor (- _y_3 (Math|Conversions|ToFloat(Integer) _index_2)))))) 1 (or (> (Math|Integer|Absolute(Integer) (Math|Float|Floor (- _x_3 (Math|Conversions|ToFloat(Integer) _index)))) _returnvalue) (> (Math|Integer|Absolute(Integer) (Math|Float|Floor (- _y_3 (Math|Conversions|ToFloat(Integer) _index_2)))) _returnvalue))))))
          (elif (or (> (Math|Integer|Absolute(Integer) (- (Math|Float|Floor (.X (Math|Vector2D|BreakVector2D (Variables|Default|GetCurrent_Chunk)))) (Math|Float|Floor _x_2))) _returnvalue_6) (> (Math|Integer|Absolute(Integer) (- (Math|Float|Floor (.Y (Math|Vector2D|BreakVector2D (Variables|Default|GetCurrent_Chunk)))) (Math|Float|Floor _y_2))) _returnvalue_6))
            ;[1 1 1] completely new position
            (for _index_3 (range _returnvalue_3 _chunk_radius)
              (for _index_4 (range _returnvalue_3 _chunk_radius)
                (CallFunction|DespawnChunk (Math|Vector2D|MakeVector2D (+ (.X (Math|Vector2D|BreakVector2D (Variables|Default|GetCurrent_Chunk))) (Math|Conversions|ToFloat(Integer) _index_3)) (+ (.Y (Math|Vector2D|BreakVector2D (Variables|Default|GetCurrent_Chunk))) (Math|Conversions|ToFloat(Integer) _index_4))))))
            (goto _label)
            (else
              ;[0 0 0] Algo for all necessary cells
              (for _index_5 (range _returnvalue_16 _returnvalue_18)
                (for _index_6 (range _returnvalue_17 _returnvalue_19)
                  (if (Math|Boolean|ANDBoolean (>= _index_5 (- (Math|Float|Floor (.X (Math|Vector2D|BreakVector2D (Variables|Default|GetCurrent_Chunk)))) _chunk_radius_3)) (<= _index_5 (+ _chunk_radius_3 (Math|Float|Floor (.X (Math|Vector2D|BreakVector2D (Variables|Default|GetCurrent_Chunk)))))) (>= _index_6 (- (Math|Float|Floor (.Y (Math|Vector2D|BreakVector2D (Variables|Default|GetCurrent_Chunk)))) _chunk_radius_3)) (<= _index_6 (+ _chunk_radius_3 (Math|Float|Floor (.Y (Math|Vector2D|BreakVector2D (Variables|Default|GetCurrent_Chunk)))))))
                    (if (> (Math|Integer|Absolute(Integer) (- (Utilities|Array|Get(acopy) (Variables|Default|GetChunk_LODs) (Utilities|Array|FindItem (Variables|Default|GetChunk_Coords) (Math|Vector2D|MakeVector2D (Math|Conversions|ToFloat(Integer) _index_5) (Math|Conversions|ToFloat(Integer) _index_6)))) (Math|Float|Ceil (Math|Float|Log (Math|Conversions|ToFloat(Integer) (Math|Integer|SelectInt (Math|Integer|SelectInt (Math|Integer|Absolute(Integer) (- _returnvalue_14 _index_5)) (Math|Integer|Absolute(Integer) (- _returnvalue_15 _index_6)) (> (Math|Integer|Absolute(Integer) (- _returnvalue_14 _index_5)) (Math|Integer|Absolute(Integer) (- _returnvalue_15 _index_6)))) 1 (or (> (Math|Integer|Absolute(Integer) (- _returnvalue_14 _index_5)) _returnvalue) (> (Math|Integer|Absolute(Integer) (- _returnvalue_15 _index_6)) _returnvalue)))) 2.0)))) 3)
                      (if (!= (Utilities|Array|FindItem (Variables|Default|GetChunk_Coords) (Math|Vector2D|MakeVector2D (Math|Conversions|ToFloat(Integer) _index_5) (Math|Conversions|ToFloat(Integer) _index_6))) -1)
                        (Utilities|Array|Add (Variables|Default|GetChunks_to_Update) (Math|Vector2D|MakeVector2D (Math|Conversions|ToFloat(Integer) _index_5) (Math|Conversions|ToFloat(Integer) _index_6)))
                        (Class|ChunkGeneratorComponent|GenerateChunk _my_chunk_generator _index_5 _index_6 (Math|Integer|Absolute(Integer) (Math|Float|Ceil (Math|Float|Log (Math|Conversions|ToFloat(Integer) (Math|Integer|SelectInt (Math|Integer|SelectInt (Math|Integer|Absolute(Integer) (- _returnvalue_14 _index_5)) (Math|Integer|Absolute(Integer) (- _returnvalue_15 _index_6)) (> (Math|Integer|Absolute(Integer) (- _returnvalue_14 _index_5)) (Math|Integer|Absolute(Integer) (- _returnvalue_15 _index_6)))) 1 (or (> (Math|Integer|Absolute(Integer) (- _returnvalue_14 _index_5)) _returnvalue) (> (Math|Integer|Absolute(Integer) (- _returnvalue_15 _index_6)) _returnvalue)))) 2.0))))
                        (Collision|LineTraceByChannel (Math|Vector|MakeVector (* _index_5 (.x _chunk_size_2)) (* _index_6 (.y _chunk_size_2)) 0.0) (Math|Vector|MakeVector (* _index_5 (.x _chunk_size_2)) (* _index_6 (.y _chunk_size_2)) 9e+04) "TraceTypeQuery1" false 0 "ForDuration" true "(R=1.000000,G=0.000000,B=0.000000,A=1.000000)" "(R=1.000000,G=0.000000,B=0.000000,A=1.000000)" 1.0)))
                    (else
                      (Class|ChunkGeneratorComponent|GenerateChunk _my_chunk_generator _index_5 _index_6 (Math|Integer|SelectInt (Math|Integer|SelectInt (Math|Integer|Absolute(Integer) (- _returnvalue_14 _index_5)) (Math|Integer|Absolute(Integer) (- _returnvalue_15 _index_6)) (> (Math|Integer|Absolute(Integer) (- _returnvalue_14 _index_5)) (Math|Integer|Absolute(Integer) (- _returnvalue_15 _index_6)))) 1 (or (> (Math|Integer|Absolute(Integer) (- _returnvalue_14 _index_5)) _returnvalue) (> (Math|Integer|Absolute(Integer) (- _returnvalue_15 _index_6)) _returnvalue))))))))
              (for _index_7 (range (- (Math|Float|Floor (.X (Math|Vector2D|BreakVector2D (Variables|Default|GetCurrent_Chunk)))) _chunk_radius_3) (+ _chunk_radius_3 (Math|Float|Floor (.X (Math|Vector2D|BreakVector2D (Variables|Default|GetCurrent_Chunk))))))
                (for _index_8 (range (- (Math|Float|Floor (.Y (Math|Vector2D|BreakVector2D (Variables|Default|GetCurrent_Chunk)))) _chunk_radius_3) (+ _chunk_radius_3 (Math|Float|Floor (.Y (Math|Vector2D|BreakVector2D (Variables|Default|GetCurrent_Chunk))))))
                  (if (not (Math|Boolean|ANDBoolean (>= _index_7 _returnvalue_16) (<= _index_7 _returnvalue_18) (>= _index_8 _returnvalue_17) (<= _index_8 _returnvalue_19)))
                    (CallFunction|DespawnChunk (Math|Vector2D|MakeVector2D (Math|Conversions|ToFloat(Integer) _index_7) (Math|Conversions|ToFloat(Integer) _index_8)))))))))))
    (:then_1
      (Variables|Default|SetCurrent_Chunk _returnvalue_13))))

(fn SpawnChunk
  (params (ChunkX :type Integer) (ChunkY :type Integer) (Vertices :type Array%20of%20Vectors) (Triangles :type Array%20of%20Integers) (Normals :type Array%20of%20Vectors) (UV0 :type Array%20of%20Vector%202D%20Structures))
  (bind _returnvalue (Math|Conversions|ToFloat(Integer) ChunkX))
  (bind _returnvalue_2 (Math|Conversions|ToFloat(Integer) ChunkY))
  (bind _chunks_to_update (Variables|Default|GetChunks_to_Update))
  (bind _returnvalue_3 (Math|Vector2D|MakeVector2D _returnvalue _returnvalue_2))
  (bind _returnvalue_4 (Utilities|Array|FindItem _chunks_to_update _returnvalue_3))
  (bind _returnvalue_5 (Game|AddComponentbyClass "/Script/Landscape_proj.AsyncPMC" false)) ; Own AsyncPMC Class
  (Class|ProceduralMeshComponent|CreateMeshSectionLinearColor _returnvalue_5 0 Vertices Triangles Normals UV0 0 0 0 0 0 (== (Utilities|Array|Length Vertices) 4225) false)
  (Rendering|Material|SetMaterial _returnvalue_5 0 "/Game/PCG_Proto/M_PMC_Auto.M_PMC_Auto")
  (Utilities|FlowControl|Sequence
    (:then_0
      (if (!= _returnvalue_4 -1)
        (CallFunction|DespawnChunk _returnvalue_3)
        (Utilities|Array|RemoveIndex _chunks_to_update _returnvalue_4)))
    (:then_1
      (Utilities|Array|Add (Variables|Default|GetChunk_Coords) _returnvalue_3)
      (Utilities|Array|Add (Variables|Default|GetChunk_LODs) (Math|Float|Floor (Math|Float|Log (- (Math|Float|Sqrt (Math|Conversions|ToFloat(Integer) (Utilities|Array|Length Triangles))) 1.0) 2.0)))
      (Utilities|Array|Add (Variables|Default|GetChunk_Refs) _returnvalue_5)
      (return))))

(fn DespawnChunk
  (params (Coords :type Vector%202D%20Structure))
  (bind _chunk_coords (Variables|Default|GetChunk_Coords))
  (bind _chunk_refs (Variables|Default|GetChunk_Refs))
  (bind _output_get (LocalVariables|Setindex (Utilities|Array|FindItem _chunk_coords Coords)))
  (if (!= _output_get -1)
    (Components|DestroyComponent (Utilities|Array|Get(acopy) _chunk_refs _output_get))
    (Utilities|IsValid (Utilities|Array|Get(acopy) _chunk_refs _output_get)
      (:Is%20Valid
        (Development|PrintString "failed to destroy chunk"))
      (:Is%20Not%20Valid
        (Utilities|Array|RemoveIndex _chunk_coords _output_get)
        (Utilities|Array|RemoveIndex (Variables|Default|GetChunk_LODs) _output_get)
        (Utilities|Array|RemoveIndex _chunk_refs _output_get)))))