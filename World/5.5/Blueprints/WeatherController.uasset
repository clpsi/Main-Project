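; Weather controller Blueprint that drives a simulated pressure field and cloud map over a tiling area sized in kilometres.
; On BeginPlay it pushes the tiling to the WeatherPainter parameter collection and starts a looping timer.
; Each tick of that timer dispatches seeded, octave-based pressure and wind generation into Weather, feeds it to cloud generation writing RT_Clouds, then advances time.
; Material-based cloud painting with a bouncing position remains unconnected.
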(event Custom|UpdateClouds
  (bind _weather (Variables|Parameters|GetWeather))
  (Class|WeatherBPL|DispatchPressureField :Output _weather :CellSize (/ (* (Variables|Parameters|GetTiling%20%28km%29) 1e+05) (Variables|/Script/Engine.TextureRenderTarget2D|GetSizeX _weather)) :SimulationTime (Variables|Calculation|GetTime) :PatternVelocity "(X=0.100000,Y=0.050000)" :Seed 12345 :BaseCells (Variables|Parameters|GetCloudSizes) :Octaves 5 :Persistence 0.5 :WindStrength 2e+01 :RotationStrength 0.5 :MaxWindStrength 2e+01 :GustStrength 2.0 :GustScale 0.01)
  (Class|WeatherBPL|DispatchCloudGeneration _weather "/Game/PCG_Proto/Weather/RT_Clouds.RT_Clouds" "(R=1.000000,G=1.000000,B=1.000000,A=1.000000)" "(R=1.000000,G=0.800000,B=0.600000,A=0.400000)" "(R=0.000000,G=0.000000,B=0.000000,A=0.000000)" "(R=0.000000,G=0.000000,B=0.000000,A=0.000000)") ; careful! default alpha != 0
  (Variables|Calculation|SetTime (+ (Variables|Calculation|GetTime) 1.0)))

(event EventBeginPlay
  (Utilities|FlowControl|Sequence
    (:then_0
      (Variables|Calculation|SetTime 0.05)
      (Rendering|Material|SetScalarParameterValue "/Game/PCG_Proto/Weather/WeatherPainter_Collection.WeatherPainter_Collection" "Tiling" (Variables|Parameters|GetTiling%20%28km%29) :!class /Script/Engine.KismetMaterialLibrary))
    (:then_1
      (Utilities|Time|SetTimerbyEvent (delegate Custom|UpdateClouds) 2.0 true true))))

(fn ConstructionScript)